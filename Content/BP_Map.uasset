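; BP_Map is a tutorial Blueprint that demonstrates Map container operations on a String-to-Integer map.
; BeginPlay switches on the MAP enum to run one example event, covering creation, add, remove, clear, lookup, keys, values, length, emptiness checks and select.
; Most examples rebuild MapStringInt with fruit-name keys, then print results to screen, often through the MapPrint helper, which loops over Keys and uses Find to show each pair.
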(event Custom|Event_ADD
  ;[0 0.9131 0.2404 0.246] Добавление элемента
  ;;[0.1874 0.2292 0.2104] ADD Добавить элемент
  (Utilities|Map|Add (Variables|Default|GetMap_String_Int) (Variables|Default|GetKey) (Variables|Default|GetElement))
  (Utilities|Map|Add (Variables|Default|GetMap_String_Int) "Яблоко" 4)
  (CallFunction|MapPrint (Variables|Default|GetMap_String_Int)))

(event Custom|Event_MakeMap
  ;[0 0.9131 0.2404 0.246] Добавление элемента
  ;;[0.1874 0.2292 0.2104] MakeMap
  ;; Перезаписывает MAP с новыми элементами
  (Variables|Default|SetMap_String_Int (Utilities|Map|MakeMap (Variables|Default|GetKey) (Variables|Default|GetElement)))
  (bind _output_get (Variables|Default|SetMap_String_Int (Utilities|Map|MakeMap "Яблоко" 3)))
  (CallFunction|MapPrint _output_get))

(event Custom|Event_VALUES
  ;[0 0.9131 0.2404 0.11] Распаковка Stuctured binding
  ;;[0.1874 0.2292 0.2104] VALUES
  (Variables|Default|SetMap_String_Int (Utilities|Map|MakeMap "Яблоко" 387 "Банан" 40))
  (bind _values (Utilities|Map|Values (Variables|Default|GetMap_String_Int)))
  (for (_array_element _array_index) _values
    (Development|PrintString (Utilities|String|Append "Element: " (Utilities|String|ToString(Integer) _array_element) " Index: " (Utilities|String|ToString(Integer) _array_index)) true true "(R=1.000000,G=0.000000,B=0.000000,A=1.000000)" 5e+01)))

(event Custom|Event_Select
  (Variables|Default|SetMap_String_Int (Utilities|Map|MakeMap "Яблоко" 3 "Банан" 3))
  (CallFunction|MapPrint (select true (Utilities|Map|MakeMap "Шаурма" 1) (Variables|Default|GetMap_String_Int))))

(event Custom|Event_CLEAR
  ;[0 0.9131 0.2404 0.178] Удаление элемента
  ;;[0.1874 0.2292 0.2104] CLEAR Удаляет все элементы
  (bind _output_get (Variables|Default|SetMap_String_Int (Utilities|Map|MakeMap "Яблоко" 3 "Банан" 3)))
  (CallFunction|MapPrint _output_get)
  (Utilities|Map|Clear (Variables|Default|GetMap_String_Int))
  (CallFunction|MapPrint (Variables|Default|GetMap_String_Int)))

(event Custom|EVENT_REMOVE%20ITEM
  ;[0 0.9131 0.2404 0.178] Удаление элемента
  ;;[0.1874 0.2292 0.2104] REMOVE ITEM
  ;; Удаляет пару ключ-значение
  (bind _output_get (Variables|Default|SetMap_String_Int (Utilities|Map|MakeMap "Яблоко" 3 "Банан" 3)))
  (CallFunction|MapPrint _output_get)
  (bind _returnvalue (Utilities|Map|Remove (Variables|Default|GetMap_String_Int) "Яблоко"))
  (Development|PrintString (Utilities|String|ToString(Boolean) _returnvalue))
  (CallFunction|MapPrint (Variables|Default|GetMap_String_Int)))

(event Custom|EVENT_CONTAINS%20ITEM
  ;[0 0.9131 0.2404 0.136] Поиск элемента
  ;;[0.1874 0.2292 0.2104] CONTAINS ITEM
  ;; Поиск элемента в MAP
  ;; Если найден элемет TRUE
  ;; Если не найден FALSE
  (bind _output_get (Variables|Default|SetMap_String_Int (Utilities|Map|MakeMap "Яблоко" 3 "Банан" 3)))
  (CallFunction|MapPrint _output_get)
  (Development|PrintString (Utilities|String|ToString(Boolean) (Utilities|Map|Contains (Variables|Default|GetMap_String_Int) "Банан"))))

(event Custom|EVENT_FIND
  ;[0 0.9131 0.2404 0.136] Поиск элемента
  ;;[0.1874 0.2292 0.2104] FIND
  ;; Поиск элемента по ключу выдает на выходе Element и логическую переменную
  (bind _output_get (Variables|Default|SetMap_String_Int (Utilities|Map|MakeMap "Яблоко" 3 "Банан" 3 "Вишня" 40)))
  (CallFunction|MapPrint _output_get)
  (Development|PrintString (Utilities|String|Append "Elemrnt: " (Utilities|String|ToString(Integer) (.Value (Utilities|Map|Find (Variables|Default|GetMap_String_Int) "Вишня"))) " Boolean: " (Utilities|String|ToString(Boolean) (.ReturnValue (Utilities|Map|Find (Variables|Default|GetMap_String_Int) "Вишня")))) true true "(R=0.000000,G=0.660000,B=1.000000,A=1.000000)" 4e+01))

(event Custom|Event_LENGTH
  ;[0 0.9131 0.2404 0.188] Длинны
  ;;[0.1874 0.2292 0.2104] LENGTH
  ;; Длинна MAP
  ;; Выдает длинну SET по чилу эементов в нем
  (bind _output_get (Variables|Default|SetMap_String_Int (Utilities|Map|MakeMap "Яблоко" 3 "Банан" 3 "Вишня" 40)))
  (CallFunction|MapPrint _output_get)
  (Development|PrintString (Utilities|String|ToString(Integer) (Utilities|Map|Length (Variables|Default|GetMap_String_Int))) true true "(R=0.000000,G=0.660000,B=1.000000,A=1.000000)" 5e+01))

(event Custom|Event_IS_EMPTY
  ;[0 0.9131 0.2404 0.11] Логические проверки
  ;;[0.1874 0.2292 0.2104] IS EMPTY
  ;; Массив пуст (Если пуст True, Если есть элементы False)
  (Development|PrintString (Utilities|String|ToString(Boolean) (Utilities|Map|IsEmpty (Variables|Default|GetMap_String_Int))) true true "(R=0.000000,G=0.660000,B=1.000000,A=1.000000)" 4e+01)
  (bind _output_get (Variables|Default|SetMap_String_Int (Utilities|Map|MakeMap "Яблоко" 3 "Банан" 3)))
  (CallFunction|MapPrint _output_get)
  (Development|PrintString (Utilities|String|ToString(Boolean) (Utilities|Map|IsEmpty (Variables|Default|GetMap_String_Int))) true true "(R=0.000000,G=0.660000,B=1.000000,A=1.000000)" 4e+01))

(event Custom|Event_IS_NOT_EMPTY
  ;[0 0.9131 0.2404 0.11] Логические проверки
  ;;[0.1874 0.2292 0.2104] IS NOT EMPTY
  ;; Массив не пуст (Если пуст False, Если есть элементы True)
  (Development|PrintString (Utilities|String|ToString(Boolean) (Utilities|Map|IsNotEmpty (Variables|Default|GetMap_String_Int))) true true "(R=0.000000,G=0.660000,B=1.000000,A=1.000000)" 4e+01)
  (bind _output_get (Variables|Default|SetMap_String_Int (Utilities|Map|MakeMap "Яблоко" 3 "Банан" 3)))
  (CallFunction|MapPrint _output_get)
  (Development|PrintString (Utilities|String|ToString(Boolean) (Utilities|Map|IsNotEmpty (Variables|Default|GetMap_String_Int))) true true "(R=0.000000,G=0.660000,B=1.000000,A=1.000000)" 4e+01))

(event Custom|Event_KEYS
  ;[0 0.9131 0.2404 0.11] Распаковка Stuctured binding
  ;;[0.1874 0.2292 0.2104] KEYS
  ;; Распаковывает MAP Выдавая название ключа и индех элемента
  (Variables|Default|SetMap_String_Int (Utilities|Map|MakeMap "Яблоко" 3 "Банан" 3))
  (bind _keys (Utilities|Map|Keys (Variables|Default|GetMap_String_Int)))
  (for (_array_element _array_index) _keys
    (Development|PrintString (Utilities|String|Append "Key: " _array_element " Index: " (Utilities|String|ToString(Integer) _array_index)) true true "(R=0.000000,G=0.660000,B=1.000000,A=1.000000)" 4e+01)))

(event EventBeginPlay
  (switch Utilities|FlowControl|Switch|SwitchonE_Map (Variables|Default|GetMAP)
    (:NewEnumerator1
      (CallFunction|EventADD))
    (:NewEnumerator15
      (CallFunction|EventMakeMap))
    (:NewEnumerator3
      (CallFunction|EventCLEAR))
    (:NewEnumerator4
      (CallFunction|EVENTREMOVEITEM))
    (:NewEnumerator6
      (CallFunction|EVENTCONTAINSITEM))
    (:NewEnumerator5
      (CallFunction|EVENTFIND))
    (:NewEnumerator7
      (CallFunction|EventLENGTH))
    (:NewEnumerator11
      (CallFunction|EventISEMPTY))
    (:NewEnumerator13
      (CallFunction|EventISNOTEMPTY))
    (:NewEnumerator12
      (CallFunction|EventKEYS))
    (:NewEnumerator16
      (CallFunction|EventVALUES))
    (:NewEnumerator14
      (CallFunction|EventSelect))))

(fn ConstructionScript)

(fn MapPrint
  (params (Map_Name :type Map%20of%20Strings%20to%20Integers))
  (Development|PrintString "MAP 
" true true "(R=1.000000,G=0.000000,B=0.579420,A=1.000000)" 4e+01)
  (bind _keys (Utilities|Map|Keys Map_Name))
  (for (_array_element _array_index) _keys
    (Development|PrintString (Utilities|String|Append "Key: " _array_element " Index: " (Utilities|String|ToString(Integer) _array_index) " Element: " (Utilities|String|ToString(Integer) (.Value (Utilities|Map|Find Map_Name _array_element)))) true true "(R=1.000000,G=0.000000,B=0.579420,A=1.000000)" 4e+01))
  (Development|PrintString " 
 
" true true "(R=0.000000,G=0.660000,B=1.000000,A=1.000000)" 4e+01)
  (return))