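; Demo Blueprint that shows the Set container operations on string sets, with Russian notes on each node.
; BeginPlay switches on the ESet enum to run one example event, covering adding, removing, queries, array conversion, Select and set algebra.
; Union, Difference and Intersection store their result in StringSetC and reprint the inputs to show they stay intact.
; The SetPrint helper converts a set to an array and prints each indexed element on screen.
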(event Custom|Event_ADD
  ;[0 0.9131 0.2404 0.246] Добавление элемента в SET
  ;;[0.1874 0.2292 0.2104] ADD Добавить элемент
  (Utilities|Set|Add (Variables|Default|GetString_Set_A) "Морковка")
  (if false
    _
    (else
      (Utilities|Set|Add (Variables|Default|GetString_Set_A) "Морковка") ; Перезапишет старое значение
    ))
  (CallFunction|SetPrint (Variables|Default|GetString_Set_A)))

(event Custom|Event_DIFFERENCE
  ;[0 0.9131 0.2404 0.136] Пересечение и Разница
  ;;[0.1874 0.2292 0.2104] DIFFERENCE разница
  ;; Удаляет из набора А элементы схожие с набором В
  (Utilities|Set|AddItems (Variables|Default|GetString_Set_A) (Utilities|Array|MakeArray "Шаурма" "Банан" "Яблоко" "Нектар"))
  (CallFunction|SetPrint (Variables|Default|GetString_Set_A))
  (Utilities|Set|AddItems (Variables|Default|GetString_Set_B) (Utilities|Array|MakeArray "Пчела" "Цветок" "Мёд" "Шаурма" "Нектар"))
  (CallFunction|SetPrint (Variables|Default|GetString_Set_B))
  (bind _result (Utilities|Set|Difference (Variables|Default|GetString_Set_A) (Variables|Default|GetString_Set_B)))
  (bind _output_get (Variables|Default|SetString_Set_C _result))
  (CallFunction|SetPrint _output_get)
  (CallFunction|SetPrint (Variables|Default|GetString_Set_A))
  (CallFunction|SetPrint (Variables|Default|GetString_Set_B)))

(event Custom|Event_IS_EMPTY
  ;[0 0.9131 0.2404 0.11] Логические проверки
  ;;[0.1874 0.2292 0.2104] IS EMPTY
  ;; Массив пуст (Если пуст True, Если есть элементы False)
  (Development|PrintString (Utilities|String|ToString(Boolean) (Utilities|Set|IsEmpty (Variables|Default|GetString_Set_A))))
  (Utilities|Set|AddItems (Variables|Default|GetString_Set_A) (Utilities|Array|MakeArray "0_Шаурма" "0_Банан" "0_Яблоко"))
  (Development|PrintString (Utilities|String|ToString(Boolean) (Utilities|Set|IsEmpty (Variables|Default|GetString_Set_A)))))

(event Custom|Event_IS_NOT_EMPTY
  ;[0 0.9131 0.2404 0.11] Логические проверки
  ;;[0.1874 0.2292 0.2104] IS NOT EMPTY
  ;; Массив не пуст (Если пуст False, Если есть элементы True)
  (Development|PrintString (Utilities|String|ToString(Boolean) (Utilities|Set|IsNotEmpty (Variables|Default|GetString_Set_A))))
  (Utilities|Set|AddItems (Variables|Default|GetString_Set_A) (Utilities|Array|MakeArray "0_Шаурма" "0_Банан" "0_Яблоко"))
  (Development|PrintString (Utilities|String|ToString(Boolean) (Utilities|Set|IsNotEmpty (Variables|Default|GetString_Set_A)))))

(event Custom|Event_TO_ARRAY
  ;[0 0.9131 0.2404 0.11] Распаковка Stuctured binding
  ;;[0.1874 0.2292 0.2104] TO ARRAY
  ;; Распаковывает, контейнер SET предоставляя контейнеру Array свои элементы
  (Utilities|Set|AddItems (Variables|Default|GetString_Set_A) (Utilities|Array|MakeArray "0_Шаурма" "0_Банан" "0_Яблоко"))
  (bind _result (Utilities|Set|ToArray (Variables|Default|GetString_Set_A)))
  (for (_array_element _array_index) _result
    (Development|PrintString (Utilities|String|Append "Index: " (Utilities|String|ToString(Integer) _array_index) " Elemrnt: " _array_element) true true "(R=0.000000,G=0.660000,B=1.000000,A=1.000000)" 4e+01)))

(event Custom|Event_Select
  (CallFunction|SetPrint (Utilities|Select :Index 0 :Option%200 (Variables|Default|GetString_Set_A) :Option%201 (Variables|Default|GetString_Set_B) :Option%202 (Utilities|Set|MakeSet "Meke"))))

(event Custom|Event_MakeSet
  ;[0 0.9131 0.2404 0.246] Добавление элемента в SET
  ;;[0.1874 0.2292 0.2104] MakeSet
  ;; Перезаписывает SET с новыми элементами
  (CallFunction|SetPrint (Variables|Default|GetString_Set_A))
  (Variables|Default|SetString_Set_A (Utilities|Set|MakeSet "Морковка" "Картошка" "Груша"))
  (CallFunction|SetPrint (Variables|Default|GetString_Set_A)))

(event Custom|Event_ADD_ITEMS
  ;[0 0.9131 0.2404 0.246] Добавление элемента в SET
  ;;[0.1874 0.2292 0.2104] ADD ITEMS Добавить набор элементов
  (Utilities|Set|AddItems (Variables|Default|GetString_Set_A) (Utilities|Array|MakeArray "Шаурма" "Банан"))
  (CallFunction|SetPrint (Variables|Default|GetString_Set_A))
  (Utilities|Set|AddItems (Variables|Default|GetString_Set_A) (Variables|Default|GetInt_Array))
  (CallFunction|SetPrint (Variables|Default|GetString_Set_A)))

(event Custom|Event_CLEAR
  ;[0 0.9131 0.2404 0.178] Удаление элемента
  ;;[0.1874 0.2292 0.2104] CLEAR Удаляет все элементы
  (Utilities|Set|AddItems (Variables|Default|GetString_Set_A) (Utilities|Array|MakeArray "Шаурма" "Банан"))
  (CallFunction|SetPrint (Variables|Default|GetString_Set_A))
  (Utilities|Set|Clear (Variables|Default|GetString_Set_A))
  (CallFunction|SetPrint (Variables|Default|GetString_Set_A)))

(event Custom|Evemt_REMOVE_ITEM
  ;[0 0.9131 0.2404 0.178] Удаление элемента
  ;;[0.1874 0.2292 0.2104] REMOVE ITEM
  ;; Удаляет элемент по значению переменной
  (Utilities|Set|AddItems (Variables|Default|GetString_Set_A) (Utilities|Array|MakeArray "Шаурма" "Банан" "Яблоко"))
  (CallFunction|SetPrint (Variables|Default|GetString_Set_A))
  (bind _returnvalue (Utilities|Set|Remove (Variables|Default|GetString_Set_A) "Шаурма"))
  (Development|PrintString (Utilities|String|ToString(Boolean) _returnvalue))
  (if _returnvalue
    (CallFunction|SetPrint (Variables|Default|GetString_Set_A))
    (else
      (CallFunction|SetPrint (Variables|Default|GetString_Set_A)))))

(event Custom|Event_REMOVE_ITEMS
  ;[0 0.9131 0.2404 0.178] Удаление элемента
  ;;[0.1874 0.2292 0.2104] REMOVE ITEMS
  ;; Удаляет перечень элементов
  (Utilities|Set|AddItems (Variables|Default|GetString_Set_A) (Utilities|Array|MakeArray "Шаурма" "Банан" "Яблоко"))
  (CallFunction|SetPrint (Variables|Default|GetString_Set_A))
  (Utilities|Set|RemoveItems (Variables|Default|GetString_Set_A) (Utilities|Array|MakeArray "Банан" "Шаурма"))
  (CallFunction|SetPrint (Variables|Default|GetString_Set_A)))

(event Custom|Event_CONTAINS_ITEM
  ;[0 0.9131 0.2404 0.136] Поиск элемента
  ;;[0.1874 0.2292 0.2104] CONTAINS ITEM
  ;; Поиск элемента в SET
  ;; Если найден элемет TRUE
  ;; Если не найден FALSE
  (Utilities|Set|AddItems (Variables|Default|GetString_Set_A) (Utilities|Array|MakeArray "Шаурма" "Банан" "Яблоко"))
  (CallFunction|SetPrint (Variables|Default|GetString_Set_A))
  (Development|PrintString (Utilities|String|ToString(Boolean) (Utilities|Set|Contains (Variables|Default|GetString_Set_A) "Банан"))))

(event Custom|Event_LENGTH
  ;[0 0.9131 0.2404 0.188] Длинны
  ;;[0.1874 0.2292 0.2104] LENGTH
  ;; Длинна SET
  ;; Выдает длинну SET по чилу эементов в нем
  (Utilities|Set|AddItems (Variables|Default|GetString_Set_A) (Utilities|Array|MakeArray "Шаурма" "Банан" "Яблоко"))
  (CallFunction|SetPrint (Variables|Default|GetString_Set_A))
  (Development|PrintString (Utilities|String|ToString(Integer) (Utilities|Set|Length (Variables|Default|GetString_Set_A))) true true "(R=1.000000,G=0.000000,B=0.579420,A=1.000000)" 4e+01))

(event Custom|Event_UNION
  ;[0 0.9131 0.2404 0.136] Объединение
  ;;[0.1874 0.2292 0.2104] UNION (Объединение)
  ;; Объеденяет SET в один не перезаписывает подаваемые SET
  (Utilities|Set|AddItems (Variables|Default|GetString_Set_A) (Utilities|Array|MakeArray "0_Шаурма" "0_Банан" "0_Яблоко"))
  (CallFunction|SetPrint (Variables|Default|GetString_Set_A))
  (Utilities|Set|AddItems (Variables|Default|GetString_Set_B) (Utilities|Array|MakeArray "1_Пчела" "1_Цветок" "1_Мёд"))
  (CallFunction|SetPrint (Variables|Default|GetString_Set_B))
  (bind _result (Utilities|Set|Union (Variables|Default|GetString_Set_A) (Variables|Default|GetString_Set_B)))
  (bind _output_get (Variables|Default|SetString_Set_C _result))
  (CallFunction|SetPrint _output_get)
  (CallFunction|SetPrint (Variables|Default|GetString_Set_A))
  (CallFunction|SetPrint (Variables|Default|GetString_Set_B)))

(event Custom|Event_INTERSECTION
  ;[0 0.9131 0.2404 0.136] Пересечение и Разница
  ;;[0.1874 0.2292 0.2104] INTERSECTION Пересечение
  ;; Удаляет из набора А элементы не схожие с набором В
  (Utilities|Set|AddItems (Variables|Default|GetString_Set_A) (Utilities|Array|MakeArray "Шаурма" "Банан" "Яблоко" "Нектар"))
  (CallFunction|SetPrint (Variables|Default|GetString_Set_A))
  (Utilities|Set|AddItems (Variables|Default|GetString_Set_B) (Utilities|Array|MakeArray "Пчела" "Цветок" "Мёд" "Шаурма" "Нектар"))
  (CallFunction|SetPrint (Variables|Default|GetString_Set_A))
  (bind _result (Utilities|Set|Intersection (Variables|Default|GetString_Set_A) (Variables|Default|GetString_Set_B)))
  (bind _output_get (Variables|Default|SetString_Set_C _result))
  (CallFunction|SetPrint _output_get)
  (CallFunction|SetPrint (Variables|Default|GetString_Set_A))
  (CallFunction|SetPrint (Variables|Default|GetString_Set_B)))

(event EventBeginPlay
  (switch Utilities|FlowControl|Switch|SwitchonE_Set (Variables|Default|GetE_Set)
    (:NewEnumerator1
      (CallFunction|EventADD))
    (:NewEnumerator2
      (CallFunction|EventADDITEMS))
    (:NewEnumerator15
      (CallFunction|EventMakeSet))
    (:NewEnumerator3
      (CallFunction|EventCLEAR))
    (:NewEnumerator4
      (CallFunction|EvemtREMOVEITEM))
    (:NewEnumerator5
      (CallFunction|EventREMOVEITEMS))
    (:NewEnumerator6
      (CallFunction|EventCONTAINSITEM))
    (:NewEnumerator7
      (CallFunction|EventLENGTH))
    (:NewEnumerator8
      (CallFunction|EventUNION))
    (:NewEnumerator9
      (CallFunction|EventDIFFERENCE))
    (:NewEnumerator10
      (CallFunction|EventINTERSECTION))
    (:NewEnumerator11
      (CallFunction|EventISEMPTY))
    (:NewEnumerator13
      (CallFunction|EventISNOTEMPTY))
    (:NewEnumerator12
      (CallFunction|EventTOARRAY))
    (:NewEnumerator14
      (CallFunction|EventSelect))))

(fn ConstructionScript)

(fn SetPrint
  (params (String_Set :type Set%20of%20Strings))
  (Development|PrintString "SET 
" true true "(R=1.000000,G=0.000000,B=0.579420,A=1.000000)" 4e+01)
  (bind _result (Utilities|Set|ToArray String_Set))
  (for (_array_element _array_index) _result
    (Development|PrintString (Utilities|String|Append "Index: " (Utilities|String|ToString(Integer) _array_index) " Elemrnt: " _array_element) true true "(R=1.000000,G=0.000000,B=0.579420,A=1.000000)" 4e+01))
  (Development|PrintString " 
 
" true true "(R=0.000000,G=0.660000,B=1.000000,A=1.000000)" 4e+01)
  (return))