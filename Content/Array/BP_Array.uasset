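; BP_Array is a teaching Blueprint that demonstrates array nodes and loop macros, with explanatory comments in Russian.
; Each custom event exercises one operation on name arrays, such as Add, Resize or copy-versus-reference Get, printing results on screen, often through the PrintArray helper.
; BeginPlay is empty, and the MapArray switch that dispatches the events is unwired, as are the loop examples.
; A separate, unwired GetItemData function reads a validated DataTable row.
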(event Custom|Event_ADD
  ;[0 0.9131 0.2404 0.063] Добавление элемента в массив
  ;;[0.1874 0.2292 0.2104] ADD Добавляет элемент в массив
  (Utilities|Array|Add (Variables|Array|GetArray_Name) "Морковка")
  (if true
    (Utilities|Array|Add (Variables|Array|GetArray_Name) "Морковка"))
  (CallFunction|PrintArray (Variables|Array|GetArray_Name)))

(event Custom|Event_ADDUNIQUE
  ;[0 0.9131 0.2404 0.063] Добавление элемента в массив
  ;;[0.1874 0.2292 0.2104] ADD UNIQUE Добавляет уникальный элемент в массив, элементы с одинаковыми именами не доблируются
  (Utilities|Array|AddUnique (Variables|Array|GetArray_Name) "Яблоко")
  (if true
    (Utilities|Array|AddUnique (Variables|Array|GetArray_Name) "Яблоко"))
  (CallFunction|PrintArray (Variables|Array|GetArray_Name)))

(event Custom|Event_Get
  ;[0 0.9131 0.2404 0.136] Поиск элемента
  (Variables|Array|SetArray_Name (Utilities|Array|MakeArray "Яблоко" "Морковка" "Виноград"))
  (CallFunction|PrintArray (Variables|Array|GetArray_Name))
  (Development|PrintString " 
 
")
  (if false
    ;;[0.1874 0.2292 0.2104] Получаем ссылку на элемент можно внести изменения
    (Development|PrintString (Utilities|String|ToString(Name) (Utilities|Array|Get(acopy) (Variables|Array|GetArray_Name) 2)) true true "(R=0.000000,G=0.660000,B=1.000000,A=1.000000)" 1e+01)
    (|SetBy-RefVar (Utilities|Array|Get(acopy) (Variables|Array|GetArray_Name) 2) "Банан")
    (CallFunction|PrintArray (Variables|Array|GetArray_Name))
    (else
      ;;[0.1874 0.2292 0.2104] Получаем копию элемента не сможем внести изменения
      (Development|PrintString (Utilities|String|ToString(Name) (Utilities|Array|Get(acopy) (Variables|Array|GetArray_Name) 2)) true true "(R=0.000000,G=0.660000,B=1.000000,A=1.000000)" 1e+01)
      ;;;[1 0 0] !!! Нельзя вызвать из копии
      (|SetBy-RefVar (Utilities|Array|Get(acopy) (Variables|Array|GetArray_Name) 2) "Банан")
      (CallFunction|PrintArray (Variables|Array|GetArray_Name)))))

(event Custom|Event_LENGTH
  ;[0 0.9131 0.2404 0.188] Длинны
  ;;[0.1874 0.2292 0.2104] LENGTH
  ;; Длинна массива
  ;; Выдает длинну массива по чилу эементов в нем
  (Development|PrintString (Utilities|String|ToString(Integer) (Utilities|Array|Length (Variables|Array|GetArray_Name))) true true "(R=1.000000,G=0.274507,B=0.000000,A=1.000000)" 2e+01)
  (Variables|Array|SetArray_Name (Utilities|Array|MakeArray "Яблоко" "Морковка" "Виноград"))
  (Development|PrintString (Utilities|String|Append " 
" (Utilities|String|ToString(Integer) (Utilities|Array|Length (Variables|Array|GetArray_Name)))) true true "(R=1.000000,G=0.274507,B=0.000000,A=1.000000)" 2e+01)
  (CallFunction|PrintArray (Variables|Array|GetArray_Name)))

(event Custom|Event_LAST_INDEX
  ;[0 0.9131 0.2404 0.188] Длинны
  ;;[0.1874 0.2292 0.2104] LAST INDEX
  ;; Последний индекс элемента в массиве
  ;; Если массив пустой то -1
  (Development|PrintString (Utilities|String|ToString(Integer) (Utilities|Array|LastIndex (Variables|Array|GetArray_Name))) true true "(R=1.000000,G=0.274507,B=0.000000,A=1.000000)" 2e+01)
  (Variables|Array|SetArray_Name (Utilities|Array|MakeArray "Яблоко" "Морковка" "Виноград"))
  (Development|PrintString (Utilities|String|Append " 
" (Utilities|String|ToString(Integer) (Utilities|Array|LastIndex (Variables|Array|GetArray_Name)))) true true "(R=1.000000,G=0.274507,B=0.000000,A=1.000000)" 2e+01)
  (CallFunction|PrintArray (Variables|Array|GetArray_Name)))

(event Custom|Event_RESIZE
  ;[0 0.9131 0.2404 0.136] Замена и перезапись
  ;;[0.1874 0.2292 0.2104] RESIZE
  ;; Устанавлмвает размер массива
  (Development|PrintString (Utilities|String|ToString(Integer) (Utilities|Array|LastIndex (Variables|Array|GetArray_Name))) true true "(R=1.000000,G=0.274507,B=0.000000,A=1.000000)" 2e+01)
  (switch string "3. Расширить массив"
    (:1.%20Установить%20размер%20массива
      (Utilities|Array|Resize (Variables|Array|GetArray_Name) 4)
      (Development|PrintString (Utilities|String|Append "Последний Index: " (Utilities|String|ToString(Integer) (Utilities|Array|LastIndex (Variables|Array|GetArray_Name))) "  Длина:  " (Utilities|String|ToString(Integer) (Utilities|Array|Length (Variables|Array|GetArray_Name)))) true true "(R=1.000000,G=0.274507,B=0.000000,A=1.000000)" 2e+01)
      (CallFunction|PrintArray (Variables|Array|GetArray_Name)))
    (:2.%20Сократить%20массив%20до%20Index
      (Variables|Array|SetArray_Name (Utilities|Array|MakeArray "Яблоко" "Морковка" "Виноград" "Шаурма"))
      (CallFunction|PrintArray (Variables|Array|GetArray_Name))
      (Utilities|Array|Resize (Variables|Array|GetArray_Name) 2)
      (CallFunction|PrintArray (Variables|Array|GetArray_Name)))
    (:3.%20Расширить%20массив
      (Variables|Array|SetArray_Name (Utilities|Array|MakeArray "Яблоко" "Морковка" "Виноград" "Шаурма"))
      (CallFunction|PrintArray (Variables|Array|GetArray_Name))
      (Utilities|Array|Resize (Variables|Array|GetArray_Name) (+ (Utilities|Array|Length (Variables|Array|GetArray_Name)) 4))
      (CallFunction|PrintArray (Variables|Array|GetArray_Name))
      (Utilities|Array|SetArrayElem (Variables|Array|GetArray_Name) 4 "Зубило")
      (CallFunction|PrintArray (Variables|Array|GetArray_Name)))))

(event Custom|Event_SetArrayElement
  ;[0 0.9131 0.2404 0.136] Замена и перезапись
  ;;[0.1874 0.2292 0.2104] Set Array Element
  ;; Перезаписать элемент по индексу
  (if false
    (Variables|Array|SetArray_Name (Utilities|Array|MakeArray "Яблоко" "Морковка" "Виноград" "Шаурма"))
    (CallFunction|PrintArray (Variables|Array|GetArray_Name))
    (Utilities|Array|SetArrayElem (Variables|Array|GetArray_Name) 1 "Зубило")
    (CallFunction|PrintArray (Variables|Array|GetArray_Name))
    (else
      ;;;[0.1874 0.2292 0.2104] Пример
      (Utilities|Array|Resize (Variables|Array|GetArray_Name) 4)
      (CallFunction|PrintArray (Variables|Array|GetArray_Name))
      (Utilities|Array|SetArrayElem (Variables|Array|GetArray_Name) 1 "Зубило")
      (CallFunction|PrintArray (Variables|Array|GetArray_Name)))))

(event Custom|Event_REVERSE
  ;[0 0.9131 0.2404 0.136] Замена и перезапись
  ;;[0.1874 0.2292 0.2104] REVERSE
  ;; Переворачивает элементы в массиве
  (bind _output_get (Variables|Array|SetArray_Name (Utilities|Array|MakeArray "Яблоко" "Морковка" "Виноград" "Шаурма")))
  (CallFunction|PrintArray _output_get)
  (Utilities|Array|Reverse (Variables|Array|GetArray_Name))
  (CallFunction|PrintArray (Variables|Array|GetArray_Name)))

(event Custom|Event_SWAP
  ;[0 0.9131 0.2404 0.136] Замена и перезапись
  ;;[0.1874 0.2292 0.2104] SWAP ARRAY ELEMENTS
  ;; Меняет элементы местами
  (bind _output_get (Variables|Array|SetArray_Name (Utilities|Array|MakeArray "Яблоко" "Морковка" "Виноград" "Шаурма")))
  (CallFunction|PrintArray _output_get)
  (Utilities|Array|Swap (Variables|Array|GetArray_Name) 0 3)
  (CallFunction|PrintArray (Variables|Array|GetArray_Name))
  (Utilities|Array|Resize (Variables|Array|GetArray_Name) (+ (Utilities|Array|Length (Variables|Array|GetArray_Name)) 4))
  (CallFunction|PrintArray (Variables|Array|GetArray_Name))
  (Utilities|Array|Swap (Variables|Array|GetArray_Name) 6)
  (CallFunction|PrintArray (Variables|Array|GetArray_Name)))

(event Custom|Event_SHUFFLE
  ;[0 0.9131 0.2404 0.136] Замена и перезапись
  ;;[0.1874 0.2292 0.2104] SHUFFLE
  ;; Перемешать элементы в массиве
  (bind _output_get (Variables|Array|SetArray_Name (Utilities|Array|MakeArray "Яблоко" "Морковка" "Виноград" "Шаурма")))
  (CallFunction|PrintArray _output_get)
  (if false
    (Utilities|Array|Shuffle (Variables|Array|GetArray_Name))
    (CallFunction|PrintArray (Variables|Array|GetArray_Name))
    (else
      (Utilities|Array|Shuffle (Variables|Array|GetArray_Name))
      (CallFunction|PrintArray (Variables|Array|GetArray_Name))
      (Utilities|Array|Shuffle (Variables|Array|GetArray_Name))
      (CallFunction|PrintArray (Variables|Array|GetArray_Name))
      (Utilities|Array|Shuffle (Variables|Array|GetArray_Name))
      (CallFunction|PrintArray (Variables|Array|GetArray_Name)))))

(event Custom|Event_INDETICAL
  ;[0 0.9131 0.2404 0.11] Логические проверки
  ;;[0.1874 0.2292 0.2104] INDETICAL
  ;; Сравнивает два массива
  ;; (Если информация одинакова True, Если информация отличается False)
  (Development|PrintString (Utilities|String|ToString(Boolean) (Utilities|Array|Identical (Variables|Array|GetArray_Name) (Variables|Array|GetArray_Name_2))))
  (Variables|Array|SetArray_Name (Utilities|Array|MakeArray "Яблоко" "Морковка" "Виноград" "Шаурма"))
  (Development|PrintString (Utilities|String|ToString(Boolean) (Utilities|Array|Identical (Variables|Array|GetArray_Name) (Variables|Array|GetArray_Name_2)))))

(event Custom|Event_IS_EMPTY
  ;[0 0.9131 0.2404 0.11] Логические проверки
  ;;[0.1874 0.2292 0.2104] IS EMPTY
  ;; Массив пуст (Если пуст True, Если есть элементы False)
  (Development|PrintString (Utilities|String|ToString(Boolean) (Utilities|Array|IsEmpty (Variables|Array|GetArray_Name))))
  (bind _output_get (Variables|Array|SetArray_Name (Utilities|Array|MakeArray "Яблоко" "Морковка" "Виноград" "Шаурма")))
  (Development|PrintString (Utilities|String|ToString(Boolean) (Utilities|Array|IsEmpty _output_get))))

(event Custom|Event_INSERT
  ;[0 0.9131 0.2404 0.063] Добавление элемента в массив
  ;;[0.1874 0.2292 0.2104] INSERT втавляет элемент в массиве по индексу
  (if false
    (Utilities|Array|Insert (Variables|Array|GetArray_Name) "Морковка")
    (else
      (Utilities|Array|Resize (Variables|Array|GetArray_Name) 4)
      (Utilities|Array|Insert (Variables|Array|GetArray_Name) "Морковка" 2)))
  (CallFunction|PrintArray (Variables|Array|GetArray_Name))
  (if true
    (Utilities|Array|Insert (Variables|Array|GetArray_Name) "Яблоко")
    (CallFunction|PrintArray (Variables|Array|GetArray_Name))))

(event Custom|Event_IS_NOT_EMPTY
  ;[0 0.9131 0.2404 0.11] Логические проверки
  ;;[0.1874 0.2292 0.2104] IS NOT EMPTY
  ;; Массив не пуст (Если пуст False, Если есть элементы True)
  (Development|PrintString (Utilities|String|ToString(Boolean) (Utilities|Array|IsNotEmpty (Variables|Array|GetArray_Name))))
  (bind _output_get (Variables|Array|SetArray_Name (Utilities|Array|MakeArray "Яблоко" "Морковка" "Виноград" "Шаурма")))
  (Development|PrintString (Utilities|String|ToString(Boolean) (Utilities|Array|IsNotEmpty _output_get))))

(event Custom|Event_IS_VALID_INDEX
  ;[0 0.9131 0.2404 0.11] Логические проверки
  ;;[0.1874 0.2292 0.2104] IS VALID INDEX
  ;; Есть ли такой индекс в массиве
  (Development|PrintString (Utilities|String|ToString(Boolean) (Utilities|Array|IsValidIndex (Variables|Array|GetArray_Name))))
  (Variables|Array|SetArray_Name (Utilities|Array|MakeArray "Яблоко" "Морковка" "Виноград" "Шаурма"))
  (Development|PrintString (Utilities|String|ToString(Boolean) (Utilities|Array|IsValidIndex (Variables|Array|GetArray_Name) 1))))

(event Custom|Event_RANDOM_ARRAY_ITEM
  ;[0 0.9131 0.2404 0.094] Рандом
  ;;[0.1874 0.2292 0.2104] RANDOM ARRAY ITEM
  ;; Выдает рандомный элемент из массива а также его индекс
  (Variables|Array|SetArray_Name (Utilities|Array|MakeArray "Яблоко" "Морковка" "Виноград" "Шаурма"))
  (for _index (range 0 4)
    (Development|PrintString (Utilities|String|Append "Index: " (Utilities|String|ToString(Integer) (.OutIndex (Utilities|Array|Random (Variables|Array|GetArray_Name)))) "  Элемент:  " (Utilities|String|ToString(Name) (.OutItem (Utilities|Array|Random (Variables|Array|GetArray_Name))))) true true "(R=0.000000,G=0.660000,B=1.000000,A=1.000000)" 2e+01)))

(event Custom|Event_Select
  (Variables|Array|SetArray_Name (Utilities|Array|MakeArray "Первый массив"))
  (CallFunction|PrintArray (Utilities|Select :Index 1 :Option%200 (Variables|Array|GetArray_Name) :Option%201 (Utilities|Array|MakeArray "Морковка" "None") :Option%202 (Utilities|Array|MakeArray "Яблоко") :Option%203 (Utilities|Array|MakeArray "Вишня" "None" "None"))))

(event Custom|Event_Make_Array
  ;[0 0.9131 0.2404 0.063] Добавление элемента в массив
  ;;[0.1874 0.2292 0.2104] Make_Array Перезаписывает массив с новыми элементами
  (CallFunction|PrintArray (Variables|Array|GetArray_Name))
  (Variables|Array|SetArray_Name (Utilities|Array|MakeArray "Яблоко" "Морковка" "Виноград"))
  (CallFunction|PrintArray (Variables|Array|GetArray_Name)))

(event Custom|Event_APPEND
  ;[0 0.9131 0.2404 0.063] Добавление элемента в массив
  ;;[0.1874 0.2292 0.2104] APPEND Объеденяет однотипные массивы массивы
  (Variables|Array|SetArray_Name (Utilities|Array|MakeArray "Яблоко" "Морковка" "Виноград"))
  (Variables|Array|SetArray_Name_2 (Utilities|Array|MakeArray "Рыба" "Мясо" "Шаурма"))
  (Utilities|Array|AppendArray (Variables|Array|GetArray_Name) (Variables|Array|GetArray_Name_2))
  (CallFunction|PrintArray (Variables|Array|GetArray_Name)))

(event Custom|Event_CLEAR
  ;[0 0.9131 0.2404 0.178] Удаление элемента
  ;;[0.1874 0.2292 0.2104] CLEAR Удаляет все элементы в массиве
  (bind _output_get (Variables|Array|SetArray_Name (Utilities|Array|MakeArray "Яблоко" "Морковка" "Виноград")))
  (CallFunction|PrintArray _output_get)
  (Development|PrintString " 
 
")
  (Utilities|Array|Clear (Variables|Array|GetArray_Name))
  (CallFunction|PrintArray (Variables|Array|GetArray_Name)))

(event Custom|EVENT_REMOVE_INDEX
  ;[0 0.9131 0.2404 0.178] Удаление элемента
  ;;[0.1874 0.2292 0.2104] REMOVE INDEX
  ;; Удалить элемент по индексу
  (bind _output_get (Variables|Array|SetArray_Name (Utilities|Array|MakeArray "Яблоко" "Морковка" "Виноград")))
  (CallFunction|PrintArray _output_get)
  (Development|PrintString " 
 
")
  (Utilities|Array|RemoveIndex (Variables|Array|GetArray_Name) 1)
  (CallFunction|PrintArray (Variables|Array|GetArray_Name)))

(event Custom|Event_REMOVE
  ;[0 0.9131 0.2404 0.178] Удаление элемента
  ;;[0.1874 0.2292 0.2104] REMOVE ITEM
  ;; Удаляет элемент по значению переменной
  (bind _output_get (Variables|Array|SetArray_Name (Utilities|Array|MakeArray "Яблоко" "Морковка" "Виноград")))
  (CallFunction|PrintArray _output_get)
  (bind _returnvalue (Utilities|Array|RemoveItem (Variables|Array|GetArray_Name) "Яблоко"))
  (Development|PrintString (Utilities|String|ToString(Boolean) _returnvalue))
  (if _returnvalue
    (CallFunction|PrintArray (Variables|Array|GetArray_Name))
    (else
      (CallFunction|PrintArray (Variables|Array|GetArray_Name)))))

(event Custom|Event_CONTAINS_ITEM
  ;[0 0.9131 0.2404 0.136] Поиск элемента
  ;;[0.1874 0.2292 0.2104] CONTAINS ITEM
  ;; Поиск элемента в массиве
  ;; Если найден элемет TRUE
  ;; Если не найден FALSE
  (Variables|Array|SetArray_Name (Utilities|Array|MakeArray "Яблоко" "Морковка" "Виноград"))
  (Development|PrintString (Utilities|String|ToString(Boolean) (Utilities|Array|ContainsItem (Variables|Array|GetArray_Name) "Морковка"))))

(event Custom|Event_FIND_ITEM
  ;[0 0.9131 0.2404 0.136] Поиск элемента
  ;;[0.1874 0.2292 0.2104] FIND ITEM
  ;; Поиск элемента
  ;; Если найден элемет выдает INDEX элемента
  ;; Если элемет не найден выдает -1
  (Variables|Array|SetArray_Name (Utilities|Array|MakeArray "Яблоко" "Морковка" "Виноград"))
  (Development|PrintString (Utilities|String|ToString(Integer) (Utilities|Array|FindItem (Variables|Array|GetArray_Name) "Морковка00")) true true "(R=0.000000,G=0.913099,B=0.240385,A=1.000000)" 2e+01))

(event EventBeginPlay)

(fn ConstructionScript)

(fn PrintArray
  (params (Array :type Array%20of%20Names))
  (Development|PrintString "Array 
" true true "(R=1.000000,G=0.053420,B=0.000000,A=1.000000)" 2e+01)
  (for (_array_element _array_index) Array
    (Development|PrintString (Utilities|String|Append "  Index:  " (Utilities|String|ToString(Integer) _array_index) "   Name:  " (Utilities|String|ToString(Name) _array_element)) true true "(R=1.000000,G=0.053420,B=0.000000,A=1.000000)" 2e+01))
  (Development|PrintString " 
 
" true true "(R=1.000000,G=0.053420,B=0.000000,A=1.000000)" 2e+01)
  (return))

(fn GetItemData
  (bind _dt_itemdata (Variables|Default|GetDT_ItemData))
  (LocalVariables|SetLocal_DataTabel (.datatable _dt_itemdata))
  (LocalVariables|SetLocal_DataRowName (.rowname _dt_itemdata))
  (Utilities|IsValid (LocalVariables|GetLocal_DataTabel)
    (:Is%20Valid
      (if (Utilities|Name|NotEqual(Name) (LocalVariables|GetLocal_DataRowName) "None")
        (bind _returnvalue (Utilities|GetDataTableRow (LocalVariables|GetLocal_DataTabel) (LocalVariables|GetLocal_DataRowName))
          (:then
            (return _returnvalue true))
          (:RowNotFound
            (return "" false)))
        (else
          (Development|PrintString (Utilities|String|Append "Ошибка: Предмет не выбран Name: " (Utilities|GetDisplayName self)) true true "(R=1.000000,G=0.000000,B=0.000000,A=1.000000)" 2e+01)
          (return "" false))))
    (:Is%20Not%20Valid
      (Development|PrintString "Ошибка: не выбрана таблица данных в предмете" true true "(R=1.000000,G=0.000000,B=0.000000,A=1.000000)" 2e+01)
      (return "" false))))