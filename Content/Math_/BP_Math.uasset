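; Math-node sandbox actor that demonstrates Blueprint math functions through debug prints, a rotating cube and a UI widget.
; BeginPlay prints an integer Wrap example, while Tick feeds game time into MakePulsatingValue to drive the cube's LerpRotator rotation.
; Player overlap with the box async-loads a soft-referenced widget once, shows it and enables Game and UI input with cursor.
; Most other math, comparison and interpolation nodes are unconnected reference examples.
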(event OnComponentBeginOverlap(Box)
  (params (OverlappedComponent :type Primitive%20Component%20Object%20Reference) (OtherActor :type Actor%20Object%20Reference) (OtherComp :type Primitive%20Component%20Object%20Reference) (OtherBodyIndex :type Integer) (bFromSweep :type Boolean) (SweepResult :type Hit%20Result%20Structure%20%28by%20ref%29))
  ;[1 1 1] Активания виджета
  (CallFunction|DebagCharacterandWidget (Variables|System|Widget|SoftRef|GetBPW_Math_SoftRef) (Game|GetPlayerCharacter 0) OtherActor)
  (Variables|System|Widget|Ref|GetBPW_Math_Ref
    (:then
      _)
    (:else
      (bind _class (Utilities|AsyncLoadClassAsset (Variables|System|Widget|SoftRef|GetBPW_Math_SoftRef))
        (:Completed
          (bind _asuser_widget (Utilities|Casting|CastToUserWidgetClass _class))
          (bind _returnvalue (UserInterface|CreateWidget _asuser_widget))
          (bind _output_get (Variables|System|Widget|Ref|SetBPW_Math_Ref _returnvalue))))))
  (UserInterface|Viewport|AddtoViewport _output_get 0)
  (CallFunction|EventGameMouse true))

(event Custom|Event_Game_Mouse
  (params (Show%20Mouse%20Cursor :type Boolean))
  ;[1 1 1] Активания виджета
  (Input|SetInputModeGameandUI (Variables|System|PC|GetPlayerController_Ref) (Variables|System|Widget|Ref|GetBPW_Math_Ref) "DoNotLock" true true)
  (Variables|/Script/Engine.PlayerController|SetbShowMouseCursor (Variables|System|PC|GetPlayerController_Ref) Show%20Mouse%20Cursor))

(event Custom|Event_FixedTurn
  ;[1 1 1] тест Fixed Turn
)

(event Custom|Event_MakePulsatingValue
  (bind _returnvalue (Utilities|Time|GetGameTimeinSeconds))
  (bind _returnvalue_2 (/ _returnvalue 25.0))
  (Development|PrintString (Utilities|String|ToString(Float) _returnvalue_2) true true "(R=0.870058,G=0.000000,B=1.000000,A=1.000000)" 0.0)
  (bind _output_get (Variables|Default|SetMake%20Pulsating%20Value (Class|KismetMathLibrary|MakePulsatingValue _returnvalue_2 (Variables|Default|GetIn%20Pulses%20Per%20Second) (Variables|Default|GetIn%20Phase))))
  (Development|PrintString (Utilities|String|ToString(Text) (Utilities|Text|ToText(Float) _output_get "HalfToEven")) true true "(R=0.064095,G=1.000000,B=0.000000,A=1.000000)" 0.0)
  (CallFunction|EventRotation))

(event Custom|Event_Rotation
  (bind _cube (Variables|Default|GetCube))
  (bind _make_pulsating_value (Variables|Default|GetMake%20Pulsating%20Value))
  (bind _returnvalue (Transformation|GetWorldRotation _cube))
  (bind _returnvalue_2 (Math|Rotator|Lerp(Rotator) (Math|Rotator|MakeRotator 0.0 (.pitch _returnvalue) 0.0) (Math|Rotator|MakeRotator 181.0 0.0 0.0) _make_pulsating_value))
  (Transformation|SetWorldRotation (Variables|Default|GetCube) (Math|Rotator|MakeRotator (.roll _returnvalue_2) (.pitch _returnvalue_2) (.yaw _returnvalue_2)) false false))

(event Custom|Event_CF)

(event EventTick
  (params (DeltaSeconds :type Float%20%28single-precision%29))
  (CallFunction|EventFixedTurn)
  (CallFunction|EventMakePulsatingValue)
  (CallFunction|EventCF))

(event EventBeginPlay
  (Variables|System|PC|SetPlayerController_Ref (Game|GetPlayerController 0))
  (Development|PrintString (Utilities|String|Append "А: " (Utilities|String|ToString(Integer) (Variables|Default|GetA_Int)) " В: " (Utilities|String|ToString(Integer) (Variables|Default|GetB_Int)) " Value: " (Utilities|String|ToString(Integer) (Variables|Default|GetValue)) " 
") true true "(R=0.962642,G=0.000000,B=1.000000,A=1.000000)" 1e+02)
  (Development|PrintString (Utilities|String|Append (Utilities|String|ToString(Integer) (Class|KismetMathLibrary|Wrap (Variables|Default|GetValue) (Variables|Default|GetA_Int) (Variables|Default|GetB_Int))) " 
") true true "(R=0.958441,G=1.000000,B=0.000000,A=1.000000)" 1e+02)
  (Development|PrintString (Utilities|String|Append "Min + (Value - Max ) = Return" " 
  " (Utilities|String|Append (Utilities|String|ToString(Integer) (Variables|Default|GetA_Int)) " + ( " (Utilities|String|ToString(Integer) (Variables|Default|GetValue)) " - " (Utilities|String|ToString(Integer) (Variables|Default|GetB_Int)) " )") " = " (Utilities|String|ToString(Integer) (+ (Variables|Default|GetA_Int) (- (Variables|Default|GetValue) (Variables|Default|GetB_Int)))) " 
") true true "(R=0.092793,G=0.156864,B=1.000000,A=1.000000)" 1e+02))

(fn ConstructionScript)

(fn DebagCharacterandWidget
  (params (SoftClassReference :type Object%20Soft%20Class%20Reference%20%28by%20ref%29) (GetCharacter :type Object%20Object%20Reference) (OtherActor :type Object%20Object%20Reference))
  (if (and (Utilities|IsValidSoftClassReference SoftClassReference) (== GetCharacter OtherActor))
    (return)))