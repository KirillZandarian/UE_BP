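; BP_Platform is a reference sandbox comparing hard, soft, class and soft class references, for generic Actor and specific cube Blueprints, with notes on their size cost.
; One custom event per variable validates it and prints its name; soft variants async-load first, and the blue cube event also calls CubeBlueRef.
; The calls to these events are disconnected, the player-checking box overlap does nothing, and the interface events and Type functions are stubs.
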(event OnComponentBeginOverlap(Box)
  (params (OverlappedComponent :type Primitive%20Component%20Object%20Reference) (OtherActor :type Actor%20Object%20Reference) (OtherComp :type Primitive%20Component%20Object%20Reference) (OtherBodyIndex :type Integer) (bFromSweep :type Boolean) (SweepResult :type Hit%20Result%20Structure%20%28by%20ref%29))
  (if (== (Game|GetPlayerCharacter 0) OtherActor)
    _))

(event Custom|Event_Actor_Ref
  ;[0 0.4573 1] Указатель на объект который находящегося на сцене (Не занимает места)
  (Utilities|IsValid (Variables|Ссылки|Ref|GetActor_Ref) ; StandartMacros 437,4 kB
    (:Is%20Valid
      (Development|PrintString (Utilities|GetDisplayName (Variables|Ссылки|Ref|GetActor_Ref))))
    (:Is%20Not%20Valid
      (Development|PrintString "Ошибка: Актер не указан" true true "(R=1.000000,G=0.000000,B=0.000000,A=1.000000)"))))

(event Custom|Event_BP_Cube_Blue_Ref
  (bind _bp_cube_blue_ref (Variables|Ссылки|Ref|GetBP_Cube_Blue_Ref))
  ;[0 0.4573 1] Передаем ссылку на объект который находиться на сцене (Нельзя указывать других актеров, непосредствено на тот класс на кого ссылается ссылка и на наследуемые классы)  (Занимает места)
  (Utilities|IsValid (Variables|Ссылки|Ref|GetBP_Cube_Blue_Ref) ; StandartMacros 437,4 kB
    (:Is%20Valid
      (Development|PrintString (Utilities|GetDisplayName _bp_cube_blue_ref))
      (Default|CubeBlueRef _bp_cube_blue_ref))
    (:Is%20Not%20Valid
      (Development|PrintString "Ошибка: Актер не указан" true true "(R=1.000000,G=0.000000,B=0.000000,A=1.000000)"))))

(event Custom|Event_Actor_SoftClassRef
  ;[0.6584 0.2122 0.6584] Указатель на класс объекта (Можно выбрать любой обьект указаного класса) (Не занимает места)
  (if (Utilities|IsValidSoftClassReference (Variables|Ссылки|SoftCalssRef|GetActor_SoftClassRef))
    (bind _class (Utilities|AsyncLoadClassAsset (Variables|Ссылки|SoftCalssRef|GetActor_SoftClassRef))
      (:then
        (Development|PrintString (Utilities|GetClassDisplayName _class)))
      (:Completed
        (bind _asactor (Utilities|Casting|CastToActorClass _class))
        (Development|PrintString (Utilities|GetClassDisplayName _asactor))))
    (else
      (Development|PrintString "Ошибка: Класс актера не выбран" true true "(R=1.000000,G=0.121763,B=0.000000,A=1.000000)"))))

(event Custom|Event_BP_Cube_Purple_SoftClassRef
  ;[0.6584 0.2122 0.6584] Передаем ссылку на класс объекта, нужно выбрать класс объекта (Нельзя указывать других актеров, непосредствено на тот класс на кого ссылается ссылка и на наследуемые классы)  (Занимает места)
  (if (Utilities|IsValidSoftClassReference (Variables|Ссылки|SoftCalssRef|GetBP_Cube_Purple_SoftClassRef))
    (bind _class (Utilities|AsyncLoadClassAsset (Variables|Ссылки|SoftCalssRef|GetBP_Cube_Purple_SoftClassRef))
      (:then
        (Development|PrintString (Utilities|GetClassDisplayName _class)))
      (:Completed
        (bind _asactor (Utilities|Casting|CastToActorClass _class))
        (Development|PrintString (Utilities|GetClassDisplayName _asactor))))
    (else
      (Development|PrintString "Ошибка: Класс актера не выбран" true true "(R=1.000000,G=0.121763,B=0.000000,A=1.000000)"))))

(event Custom|Event_Actor_SoftRef
  ;[0.3005 1 1] Мягкая указатель на объект который находиться на сцене. Можно выбрать объект который находиться на сцене через детали переменной (Не занимает места)
  (if (Utilities|IsValidSoftObjectReference (Variables|Ссылки|SoftRef|GetActor_SoftRef))
    (bind _object (Utilities|AsyncLoadAsset (Variables|Ссылки|SoftRef|GetActor_SoftRef))
      (:then
        (Development|PrintString (Utilities|GetDisplayName _object)))
      (:Completed
        (bind _asactor (Utilities|Casting|CastToActor _object))
        (Development|PrintString (Utilities|GetDisplayName _asactor))))
    (else
      (Development|PrintString "Ошибка: Актер не указан" true true "(R=1.000000,G=0.000000,B=0.000000,A=1.000000)"))))

(event Custom|Event_BP_Cube_TurquoiseBlue_SoftRef
  ;[0.3005 1 1] Передаем ссылку на объект который находиться на сцене. Можно выбрать объект который находиться на сцене через детали переменной (Нельзя указывать других актеров, непосредствено на тот класс на кого ссылается ссылка и на наследуемые классы)  (Не занимает места)
  (if (Utilities|IsValidSoftObjectReference (Variables|Ссылки|SoftRef|GetBP_Cube_TurquoiseBlue_SoftRef))
    (bind _object (Utilities|AsyncLoadAsset (Variables|Ссылки|SoftRef|GetBP_Cube_TurquoiseBlue_SoftRef))
      (:then
        (Development|PrintString (Utilities|GetDisplayName _object)))
      (:Completed
        (bind _asactor (Utilities|Casting|CastToActor _object))
        (Development|PrintString (Utilities|GetDisplayName _asactor))))
    (else
      (Development|PrintString "Ошибка: Актер не указан" true true "(R=1.000000,G=0.000000,B=0.000000,A=1.000000)"))))

(event Custom|Event_Actor_ClassRef
  ;[0.0999 0 0.5029] Указатель на класс объекта (Можно выбрать любой обьект указаного класса) (Занимает места)
  (if (Utilities|IsValidClass (Variables|Ссылки|ClassRef|GetActor_ClassRef))
    (Development|PrintString (Utilities|GetClassDisplayName (Variables|Ссылки|ClassRef|GetActor_ClassRef)))
    (else
      (Development|PrintString "Ошибка: Класс актера не выбран" true true "(R=1.000000,G=0.121763,B=0.000000,A=1.000000)"))))

(event Custom|Event_BP_Cube_Lilac_RefClass
  ;[0.0999 0 0.5029] Передаем ссылку на класс объекта, нужно выбрать класс объекта (Нельзя указывать других актеров, непосредствено на тот класс на кого ссылается ссылка и на наследуемые классы)  (Занимает места)
  (if (Utilities|IsValidClass (Variables|Ссылки|Class_Ref|GetBP_Cube_Lilac_RefClass))
    (Development|PrintString (Utilities|GetClassDisplayName (Variables|Ссылки|Class_Ref|GetBP_Cube_Lilac_RefClass)))
    (else
      (Development|PrintString "Ошибка: Класс актера не выбран" true true "(R=1.000000,G=0.121763,B=0.000000,A=1.000000)"))))

(event Event11Type
  (params (Int :type Integer))
  ;[0 0.402 0.9131] Interface
)

(event Event1Type
  ;[0 0.402 0.9131] Interface
)

(fn ConstructionScript)

(fn 2Type
  (return 0))

(fn 3Type
  (params (int :type Integer))
  (return 0))