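; BP_Platform_BPI is a trigger platform that calls a Blueprint Interface message on a referenced actor when the player character overlaps its box.
; A reusable check, DoesIsActorAndInterface, validates the reference and interface implementation, branching to Yes BPI, No BPI or No Ref.
; Success sends BPI1Message, while either failure prints a Russian error.
; Disconnected nodes hold other interface-call examples, including one with a return value.
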(event OnComponentBeginOverlap(Box)
  (params (OverlappedComponent :type Primitive%20Component%20Object%20Reference) (OtherActor :type Actor%20Object%20Reference) (OtherComp :type Primitive%20Component%20Object%20Reference) (OtherBodyIndex :type Integer) (bFromSweep :type Boolean) (SweepResult :type Hit%20Result%20Structure%20%28by%20ref%29))
  (if (== (Game|GetPlayerCharacter 0) OtherActor)
    (bind _outputpin (Utilities|DoesIsActorandInterface (Variables|Ссылки|Ref|GetActor_Ref) (Variables|Default|GetInterface))
      (:Yes%20BPI
        (Class|BPIYYY|BPI1(Message) _outputpin))
      (:No%20BPI
        (Development|PrintString "Ошибка: Нет Интерфейса у данного объекта" true true "(R=1.000000,G=0.041194,B=0.000000,A=1.000000)" 1e+01))
      (:No%20Ref
        (Development|PrintString "Ошибка: Объект не выбран" true true "(R=1.000000,G=0.000000,B=0.015278,A=1.000000)" 1e+01)))))

(fn ConstructionScript)