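; BP_Platform_SoftRef_ is a trigger platform that messages a soft-referenced object when the player steps on it.
; Box overlap by player 0 validates ActorSoftRef and async loads it, avoiding a hard reference.
; The loaded object must implement both BPI_Cude and BPI_Cube_SoftRef to receive CubeDataMessage; otherwise, or when the reference is invalid, it prints a Russian error.
; A CubeSoftRefMessage call is left unconnected.
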(event OnComponentBeginOverlap(Box)
  (params (OverlappedComponent :type Primitive%20Component%20Object%20Reference) (OtherActor :type Actor%20Object%20Reference) (OtherComp :type Primitive%20Component%20Object%20Reference) (OtherBodyIndex :type Integer) (bFromSweep :type Boolean) (SweepResult :type Hit%20Result%20Structure%20%28by%20ref%29))
  (if (== (Game|GetPlayerCharacter 0) OtherActor)
    (if (Utilities|IsValidSoftObjectReference (Variables|Ссылки|SoftRef|GetActor_SoftRef))
      (bind _object (Utilities|AsyncLoadAsset (Variables|Ссылки|SoftRef|GetActor_SoftRef))
        (:Completed
          (if (and (Utilities|DoesObjectImplementInterface _object "/Game/Ref/Platform/BPI_Cude.BPI_Cude_C") (Utilities|DoesObjectImplementInterface _object "/Game/Ref/Platform/BPI_Cube_SoftRef.BPI_Cube_SoftRef_C"))
            (Class|BPICude|CubeData(Message) _object)
            (else
              (Development|PrintString "Ошибка: Нет Интерфейса" true true "(R=1.000000,G=0.209649,B=0.000000,A=1.000000)" 1e+01)))))
      (else
        (Development|PrintString "Ошибка: Объект не выбран" true true "(R=1.000000,G=0.000000,B=0.156486,A=1.000000)" 1e+01)))))

(fn ConstructionScript)