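; BP_Structure is a demo Blueprint for structs and Data Tables that changes the material on its Cube from table data.
; GetDataNameID looks up a row by name in DT_Structure, async-loads its soft Material reference and applies it as a Material Instance.
; GetDataEnum and BeginPlay are empty.
; Unconnected example nodes, some with Russian notes, show struct break/make, row handles, table queries and an enum-to-row-name lookup.
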(event EventBeginPlay)

(event EventGetDataNameID
  (params (RowName :type Name :default "None") (S_Structure :type S%20Structure%20Structure))
  (bind _returnvalue (Utilities|GetDataTableRow "/Game/Structure/DT_Structure.DT_Structure" RowName)
    (:then
      (bind _object (Utilities|AsyncLoadAsset (Utilities|Struct|BreakS_Structure _returnvalue))
        (:Completed
          (bind _asmaterial_instance (Utilities|Casting|CastToMaterialInstance _object))
          (Rendering|Material|SetMaterial (Variables|Default|GetCube) 0 _asmaterial_instance))))))

(event EventGetDataEnum
  (params (E_Enum :type E_Enum%20Enum :default "NewEnumerator3") (E_Structure :type E_Structure%20Enum :default "NewEnumerator0")))

(fn ConstructionScript)