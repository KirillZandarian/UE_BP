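; Cube actor that shows an enum-selected color and passes its enum and data table row name to other actors when hit.
; On BeginPlay it looks up the enum in a map to set the cube's material; an unconnected Switch version remains in the graph.
; On Hit it async-loads two soft-referenced targets and sends interface messages: row name and enum data to the first, enum data to the second.
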(event EventBeginPlay
  (bind _e_enum (Variables|Default|GetE_Enum))
  (bind _map_e_enum (Variables|Default|GetMap_E_Enum))
  (bind (_value _returnvalue) (Utilities|Map|Find _map_e_enum _e_enum))
  (Utilities|FlowControl|Sequence
    (:then_1
      ;[0.1271 0.1651 0.4844] С использованием контейнера MAP
      ; !!! 1. Необходимо указать в контейнере цвета
      ; !!! 2. В перечеслителе первая строка с именем None
      (if _returnvalue
        (Rendering|Material|SetMaterial (Variables|Default|GetCube) 0 _value)))))

(event Collision|EventHit
  (params (MyComp :type Primitive%20Component%20Object%20Reference) (Other :type Actor%20Object%20Reference) (OtherComp :type Primitive%20Component%20Object%20Reference) (bSelfMoved :type Boolean) (HitLocation :type Vector :default "0, 0, 0") (HitNormal :type Vector :default "0, 0, 0") (NormalImpulse :type Vector :default "0, 0, 0") (Hit :type Hit%20Result%20Structure%20%28by%20ref%29))
  (Utilities|FlowControl|Sequence
    (:then_0
      (if (Utilities|IsValidSoftObjectReference (Variables|Default|GetS_Actor))
        (bind _object (Utilities|AsyncLoadAsset (Variables|Default|GetS_Actor))
          (:Completed
            (Class|BPIStructure|GetDataNameID(Message) _object (.rowname (Variables|Default|GetDT_Structure%20%28Data%20Tabler%20Row%20Handle%29)))
            (Class|BPIEEnum|GetDataEnum(Message) _object (Variables|Default|GetE_Enum) (Variables|Default|GetE_Structure))))))
    (:then_1
      (if (Utilities|IsValidSoftObjectReference (Variables|Default|GetE_Actor))
        (bind _object_2 (Utilities|AsyncLoadAsset (Variables|Default|GetE_Actor))
          (:Completed
            (Class|BPIEEnum|GetDataEnum(Message) _object_2 (Variables|Default|GetE_Enum) "NewEnumerator0")))))))

(fn ConstructionScript)