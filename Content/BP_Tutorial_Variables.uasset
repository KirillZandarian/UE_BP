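; Tutorial actor, annotated in Russian, that demonstrates Blueprint variable types and ways to reference actors and classes.
; A Variables graph shows Set, Make, Break and Split nodes for primitives, structs and hard or soft references.
; EventGraph examples get or spawn cubes via direct, class and async-loaded soft references, mostly printing through DEBAGPrintActor, which compares direct, interface and cast access.
; All examples are unwired and BeginPlay is empty, so nothing runs.
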(event EventBeginPlay)

(fn ConstructionScript)

(fn DEBAGPrintActor
  (params (InputPin :type Actor%20Object%20Reference) (Local_TextColor1 :type Linear%20Color%20Structure))
  (LocalVariables|SetLoacal_Actor InputPin)
  (LocalVariables|SetLocal_TextColor Local_TextColor1)
  (Utilities|IsValid (LocalVariables|GetLoacal_Actor)
    (:Is%20Valid
      (Development|PrintString (Utilities|String|Append "На прямую: " (Utilities|GetDisplayName (LocalVariables|GetLoacal_Actor))) true true (LocalVariables|GetLocal_TextColor) 1e+01)
      (bind _actor_ref (Class|BPIRefCUbe|CubRef(Message) (LocalVariables|GetLoacal_Actor)))
      (Development|PrintString (Utilities|String|Append "Через интерфайс: " (Utilities|GetDisplayName _actor_ref)) true true (LocalVariables|GetLocal_TextColor) 1e+01)
      (bind _asbp_red_cube_soft_ref (Utilities|Casting|CastToBP_RedCube_SoftRef (LocalVariables|GetLoacal_Actor)))
      (Development|PrintString (Utilities|String|Append "Через Каст: " (Utilities|GetDisplayName _asbp_red_cube_soft_ref)) true true (LocalVariables|GetLocal_TextColor) 1e+01))))