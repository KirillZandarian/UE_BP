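; BP_Event is a test actor for custom events, event dispatchers and a clamped HP function.
; Custom events change CurrHP either by raw addition or through the HP clamp, printing values for comparison.
; Player overlap with the Box broadcasts EventDisOverlap with the player's name, adds a widget and shows the cursor; leaving broadcasts "None".
; Hit leads only to a DoOnce, and the test calls and EventDisHP binding are left disconnected.
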(event OnComponentBeginOverlap(Box)
  (params (OverlappedComponent :type Primitive%20Component%20Object%20Reference) (OtherActor :type Actor%20Object%20Reference) (OtherComp :type Primitive%20Component%20Object%20Reference) (OtherBodyIndex :type Integer) (bFromSweep :type Boolean) (SweepResult :type Hit%20Result%20Structure%20%28by%20ref%29))
  (bind _returnvalue (Game|GetPlayerCharacter 0))
  (if (== _returnvalue OtherActor)
    (Default|CallEventDisOverlap (Utilities|GetDisplayName _returnvalue))
    (bind _returnvalue_2 (UserInterface|CreateWidget "/Game/Delagate/NewWidgetBlueprint.NewWidgetBlueprint_C"))
    (UserInterface|Viewport|AddtoViewport _returnvalue_2 0)
    (Variables|/Script/Engine.PlayerController|SetbShowMouseCursor (Game|GetPlayerController 0) true)))

(event OnComponentEndOverlap(Box)
  (params (OverlappedComponent :type Primitive%20Component%20Object%20Reference) (OtherActor :type Actor%20Object%20Reference) (OtherComp :type Primitive%20Component%20Object%20Reference) (OtherBodyIndex :type Integer))
  (if (== (Game|GetPlayerCharacter 0) OtherActor)
    (Default|CallEventDisOverlap "None")))

(event Custom|Event_AS_HP_1
  (params (HP :type Integer))
  (Variables|Default|SetCurr_HP (+ (Variables|Default|GetCurr_HP) HP)))

(event Custom|Event_AS_HP_2
  (params (HP :type Integer))
  (bind _new_hp (CallFunction|HP (Variables|Default|GetCurr_HP) HP (Variables|Default|GetMax_HP)))
  (bind _output_get (Variables|Default|SetCurr_HP _new_hp)))

(event Custom|Event_One
  (bind _output_get (Variables|Default|SetCurr_HP 10))
  (Development|PrintString (Utilities|String|Append "Первое значение:  " (Utilities|String|ToString(Integer) _output_get)) true true "(R=0.174185,G=0.133474,B=1.000000,A=1.000000)" 1e+01)
  (CallFunction|EventASHP1 10)
  (Development|PrintString (Utilities|String|Append "Второе значение:  " (Utilities|String|ToString(Integer) (Variables|Default|GetCurr_HP))) true true "(R=0.000000,G=0.660000,B=1.000000,A=1.000000)" 1e+01)
  (CallFunction|EventASHP2 -5)
  (Development|PrintString (Utilities|String|Append "Третье значение:  " (Utilities|String|ToString(Integer) (Variables|Default|GetCurr_HP))) true true "(R=0.272618,G=1.000000,B=0.000000,A=1.000000)" 1e+01))

(event Custom|Event_Two
  (params (HP :type Integer))
  (Variables|Default|SetCurr_HP HP)
  (Development|PrintString (Utilities|String|Append "Первое значение:  " (Utilities|String|ToString(Integer) HP)))
  (bind _new_hp (CallFunction|HP (Variables|Default|GetCurr_HP) HP (Variables|Default|GetMax_HP)))
  (Variables|Default|SetCurr_HP _new_hp))

(event Collision|EventHit
  (params (MyComp :type Primitive%20Component%20Object%20Reference) (Other :type Actor%20Object%20Reference) (OtherComp :type Primitive%20Component%20Object%20Reference) (bSelfMoved :type Boolean) (HitLocation :type Vector :default "0, 0, 0") (HitNormal :type Vector :default "0, 0, 0") (NormalImpulse :type Vector :default "0, 0, 0") (Hit :type Hit%20Result%20Structure%20%28by%20ref%29))
  (if (== (Game|GetPlayerCharacter 0) Other)
    (Utilities|FlowControl|DoOnce false)))

(fn ConstructionScript)

(fn HP
  (params (curr_HP :type Integer) (HP :type Integer) (max_Hp :type Integer))
  (return (Math|Integer|Clamp(Integer) (+ curr_HP HP) 0 max_Hp)))