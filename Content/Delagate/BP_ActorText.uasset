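; Text display actor that shows the overlap name broadcast by a referenced actor through an event dispatcher.
; On BeginPlay it validates the Actor reference and binds a custom event to its EventDisOverlap dispatcher.
; That event writes the received name to the TextRender component and prints it.
; Separate dispatcher handlers also exist: one prints the name again, and one for a second actor reference is empty.
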(event EventDisOverlap(Actor)
  (params (NameOverlap :type String))
  (Development|PrintString NameOverlap))

(event EventDisOverlap(Actor_0)
  (params (NameOverlap :type String)))

(event Custom|EventDis_Overlap_Event
  (params (NameOverlap :type String))
  (Rendering|Components|TextRender|SetText (Variables|Default|GetTextRender) (Utilities|Text|ToText(String) NameOverlap))
  (Development|PrintString (stale EventDisOverlap(Actor) NameOverlap)))

(event EventBeginPlay
  (Utilities|IsValid (Variables|Default|GetActor)
    (:Is%20Valid
      (EventDispatchers|AssignEventDisOverlap (Variables|Default|GetActor) (delegate Custom|EventDis_Overlap_Event)))))

(fn ConstructionScript)