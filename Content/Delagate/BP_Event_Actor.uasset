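; Demo actor that catalogs Blueprint event types and the Event Dispatcher (Observer) pattern, with notes in Russian.
; BeginPlay raises the load-game event, which broadcasts the dispatcher; a custom event also broadcasts its parameter.
; Hit, Reset and EndPlay print debug text, and Event_Ev shows delegates feeding timers and a window-close callback.
; Bind, unbind, damage and level-reset examples are unwired, and most other events are empty stubs.
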(event Custom|Event_Ev
  ;[1 1 1] Widget
  (Class|WidgetBlueprintLibrary|SetWindowTitleBaronCloseClickedDelegate (delegate Custom|Event_Ev))
  ;[1 1 1] Timers
  (bind _returnvalue (Utilities|Time|SetTimerbyEvent (delegate Custom|Event_Ev) 0.0))
  (Variables|Default|SetTimer _returnvalue)
  (bind _returnvalue_2 (Class|KismetSystemLibrary|SetTimerforNextTickDelegate (delegate Custom|Event_Ev)))
  (Variables|Default|SetTimer _returnvalue_2))

(event Custom|Event_Call_In_Editor
  ;[1 1 1 0.058] DELEGATE EVENT
)

(event Custom|Event_Subscriber_2
  (params (NewParam :type Integer))
  ;[1 1 1] Подписчик канала BP_Subscriber
  ;;[1 1 1] Уведомление
)

(event Custom|Event_Subscriber_1
  (params (NewParam :type Integer))
  ;[1 1 1] Подписчик канала BP_Subscriber
  ;;[1 1 1] Уведомление
)

(event Custom|Event_Custom_2
  ;[1 1 1 0.058] DELEGATE EVENT
)

(event Custom|OnActorHit_Event
  (params (SelfActor :type Actor%20Object%20Reference) (OtherActor :type Actor%20Object%20Reference) (NormalImpulse :type Vector) (Hit :type Hit%20Result%20Structure%20%28by%20ref%29))
  (Development|PrintString (Utilities|GetDisplayName OtherActor)))

(event Custom|EventDispatcher_Event
  (params (NewParam :type Integer))
  ;[1 1 1 0.084] DELEGATE EVENT DISPATCHER
  ;;[1 1 1] Уведомление
)

(event Custom|Event_Inputs
  (params (int :type Integer))
  ;[1 0 0 0.5] DELEGATE EVENT DISPATCHER  ПАТТЕРН OBSERVER
  ;;[0.3292 0.8385 0.5757 1 16] Поступило уведомление работаем
)

(event Custom|Event_%20LoadGame
  ;[1 0 0 0.5] DELEGATE EVENT
  ;;[0 0 0 0 16] Произошло событие загрузка игры
  ;[1 0 0 0.5] DELEGATE EVENT DISPATCHER  ПАТТЕРН OBSERVER
  ;;[0.3292 0.8385 0.5757] observer-наблюдатель
  ;; Сижу слежу :)
  (Default|CallEventDispatcher))

(event Custom|Event_Event
  (params (NewParam :type Integer))
  ;[1 1 1] Какоето событие
  ;[1 1 1] Телеграмм канал BP_Telegram
  ;;[1 1 1] observer-наблюдатель
  (Default|CallEventDispatcher NewParam))

(event EventBeginPlay
  ;[1 0 0 0.5] DELEGATE EVENT
  ;;[0.3292 0.8385 0.5757] Игра запустилась
  (CallFunction|EventLoadGame))

(event MouseInput|EventActorBeginCursorOver
  ;[1 1 1] Событие навидение курсора
)

(event Collision|EventActorBeginOverlap
  (params (OtherActor :type Actor%20Object%20Reference))
  ;[1 1 1] События перекрытия (Работает если есть колизия "Бокс, сфера, капсула")
)

(event MouseInput|EventActorEndCursorOver
  ;[1 1 1] Событие навидение курсора
)

(event Collision|EventActorEndOverlap
  (params (OtherActor :type Actor%20Object%20Reference))
  ;[1 1 1] События перекрытия (Работает если есть колизия "Бокс, сфера, капсула")
)

(event MouseInput|EventActorOnClicked
  (params (ButtonPressed :type Key%20Structure :default "None")))

(event EventActorOnReleased
  (params (ButtonReleased :type Key%20Structure :default "None")))

(event Game|Damage|EventAnyDamage
  (params (Damage :type Float%20%28single-precision%29) (DamageType :type Damage%20Type%20Object%20Reference) (InstigatedBy :type Controller%20Object%20Reference) (DamageCauser :type Actor%20Object%20Reference))
  ;[1 1 1] События повреждения
)

(event EventAsyncPhysicsTick
  (params (DeltaSeconds :type Float%20%28single-precision%29) (SimSeconds :type Float%20%28single-precision%29))
  ;[1 1 1] Вызывается при каждом тики физики
)

(event EventActorOnInputTouchBegin
  (params (FingerIndex :type ETouchIndex%20Enum :default "Touch1"))
  ;[1 1 1] События для сенсоров (Экранов и тд)
)

(event EventDestroyed
  ;[1 1 1] Событие уничтожено (Сробатывает когда актер уничтожен) переведена в событие End Play
)

(event EventEndPlay
  (params (EndPlayReason :type EEndPlayReason%20Enum :default "Destroyed"))
  ;[1 1 1] Событие воспроизводиться в конце (Пример когда актер удален)
  (Development|PrintString (Utilities|String|EnumtoString EndPlayReason))
  (switch Utilities|FlowControl|Switch|SwitchonEEndPlayReason EndPlayReason
    (:Destroyed
      (Actor|DestroyActor))))

(event EventActorOnInputTouchEnd
  (params (FingerIndex :type ETouchIndex%20Enum :default "Touch1"))
  ;[1 1 1] События для сенсоров (Экранов и тд)
)

(event Collision|EventHit
  (params (MyComp :type Primitive%20Component%20Object%20Reference) (Other :type Actor%20Object%20Reference) (OtherComp :type Primitive%20Component%20Object%20Reference) (bSelfMoved :type Boolean) (HitLocation :type Vector :default "0, 0, 0") (HitNormal :type Vector :default "0, 0, 0") (NormalImpulse :type Vector :default "0, 0, 0") (Hit :type Hit%20Result%20Structure%20%28by%20ref%29))
  ;[1 1 1] Событие столкновения (Работает если есть с чем столкнуться)
  (Development|PrintString (Utilities|GetDisplayName Other)))

(event EventOnBecomeViewTarget
  (params (PC :type Player%20Controller%20Object%20Reference))
  ;[1 1 1] Когда этот актер становится целью просмотра для данного PlayerController
)

(event EventOnEndViewTarget
  (params (PC :type Player%20Controller%20Object%20Reference))
  ;[1 1 1] Когда этот актер становится целью просмотра для данного PlayerController
)

(event EventOnReset
  ;[1 1 1] Сробатывает при сбросе уровня
  (Development|PrintString "Reset Actor"))

(event Game|Damage|EventPointDamage
  (params (Damage :type Float%20%28single-precision%29) (DamageType :type Damage%20Type%20Object%20Reference) (HitLocation :type Vector :default "0, 0, 0") (HitNormal :type Vector :default "0, 0, 0") (HitComponent :type Primitive%20Component%20Object%20Reference) (BoneName :type Name :default "None") (ShotFromDirection :type Vector :default "0, 0, 0") (InstigatedBy :type Controller%20Object%20Reference) (DamageCauser :type Actor%20Object%20Reference) (HitInfo :type Hit%20Result%20Structure%20%28by%20ref%29))
  ;[1 1 1] События повреждения
)

(event Game|Damage|EventRadialDamage
  (params (DamageReceived :type Float%20%28single-precision%29) (DamageType :type Damage%20Type%20Object%20Reference) (Origin :type Vector :default "0, 0, 0") (HitInfo :type Hit%20Result%20Structure%20%28by%20ref%29) (InstigatedBy :type Controller%20Object%20Reference) (DamageCauser :type Actor%20Object%20Reference))
  ;[1 1 1] События повреждения
)

(event EventTick
  (params (DeltaSeconds :type Float%20%28single-precision%29))
  ;[1 0 0] Тихая система (Тик) (Вызывается в каждом кадре игрового процесса)
)

(event EventActorOnInputTouchEnter
  (params (FingerIndex :type ETouchIndex%20Enum :default "Touch1"))
  ;[1 1 1] События для сенсоров (Экранов и тд)
)

(event EventActorOnInputTouchLeave
  (params (FingerIndex :type ETouchIndex%20Enum :default "Touch1"))
  ;[1 1 1] События для сенсоров (Экранов и тд)
)

(fn ConstructionScript)

(fn Function)