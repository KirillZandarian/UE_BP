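; BP_Master_Items is a base item actor meant to take its data and mesh from a DataTable row handle.
; BeginPlay currently only async-loads a soft asset reference, casts it to DataTable and prints its name.
; DataFromTheSobject validates the table and row, returning the row with a success flag.
; Its use to async-load the static mesh, or destroy the actor on failure, is disconnected and never runs.
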(event EventBeginPlay
  (bind _object (Utilities|AsyncLoadAsset (Variables|Default|GetAsset))
    (:Completed
      (bind _asdata_table (Utilities|Casting|CastToDataTable _object))
      (Development|PrintString (Utilities|GetDisplayName _asdata_table)))))

(fn ConstructionScript)

(fn DatafromtheSobject
  (bind _dataitems (Variables|Data|GetDataItems))
  (LocalVariables|SetLocal_DataTable (.datatable _dataitems))
  (LocalVariables|SetLocal_RowName (.rowname _dataitems))
  (Utilities|IsValid (LocalVariables|GetLocal_DataTable)
    (:Is%20Valid
      (if (not (== (LocalVariables|GetLocal_RowName) ""))
        (bind _returnvalue (Utilities|GetDataTableRow (LocalVariables|GetLocal_DataTable) (LocalVariables|GetLocal_RowName))
          (:then
            (return _returnvalue true))
          (:RowNotFound
            (return "" false)))
        (else
          (Development|PrintString (Utilities|String|Append "Ошибка: Не выбран предмет: " (Utilities|GetDisplayName self)) true true "(R=1.000000,G=0.000000,B=0.000000,A=1.000000)" 4e+01)
          (return "" false))))
    (:Is%20Not%20Valid
      (Development|PrintString "Ошибка: Не выбрана таблица данных" true true "(R=1.000000,G=0.000000,B=0.000000,A=1.000000)" 4e+01)
      (return "" false))))