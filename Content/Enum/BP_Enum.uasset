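; BP_Enum is an enum tutorial Blueprint that recolors its Cube mesh based on an EEnum color value.
; The GetDataEnum event stores the incoming value, looks it up in the MapEEnum map and applies the found material to the Cube.
; An unconnected Switch-based alternative and various loose enum conversion and switch nodes remain in the graph as examples.
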(event EventGetDataEnum
  (params (E_Enum :type E_Enum%20Enum :default "NewEnumerator3"))
  (Variables|Default|SetE_Enum E_Enum)
  (Utilities|FlowControl|Sequence
    (:then_1
      ;[0.1271 0.1651 0.4844] С использованием контейнера MAP
      ; !!! 1. Необходимо указать в контейнере цвета
      ; !!! 2. В перечеслителе первая строка с именем None
      (if (.ReturnValue (Utilities|Map|Find (Variables|Default|GetMap_E_Enum) (Variables|Default|GetE_Enum)))
        (Rendering|Material|SetMaterial (Variables|Default|GetCube) 0 (.Value (Utilities|Map|Find (Variables|Default|GetMap_E_Enum) (Variables|Default|GetE_Enum))))))))

(fn ConstructionScript)